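; Game instance for multiplayer that manages menu widgets and session hosting, joining and teardown.
; Show events create and cache widgets, most re-adding a valid cached one to the viewport.
; LaunchLobby creates a session and opens "lobby" as a listen server; JoinServer joins a given search result, both behind a loading screen.
; Session, network and travel failures route to DisplayErrorMessage, but it and both error-to-string helpers are empty stubs here.
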(event Custom|LaunchLobby
  (params (NumberOfPlayers :type Integer) (EnableLAN? :type Boolean) (ServerName :type Text))
  ;[1 1 1] Enter the fun zone
  (Variables|ServerSettings|SetMaxPlayers NumberOfPlayers)
  (Variables|ServerSettings|SetServerName ServerName)
  (CallFunction|ShowLoadingScreen)
  (|Session (Game|GetPlayerController 0) (Variables|ServerSettings|GetMaxPlayers) EnableLAN?
    (:OnSuccess
      (Game|OpenLevel(byName) "lobby" true "listen"))
    (:OnFailure
      (Utilities|DisplayErrorMessage "\"You look tired, you should go to bed.\""))))

(event Custom|ShowMainMenu
  (bind _returnvalue (Game|GetPlayerController 0))
  ;[1 1 1] Take it from the top, dawg
  (Utilities|IsValid (Variables|Widget|GetMainMenuWID)
    (:Is%20Valid
      (UserInterface|Viewport|AddtoViewport (Variables|Widget|GetMainMenuWID) 0)
      (Variables|/Script/Engine.PlayerController|SetbShowMouseCursor _returnvalue true))
    (:Is%20Not%20Valid
      (bind _returnvalue_2 (UserInterface|CreateWidget "/Game/Multiplayer/UI/MainMenu/MainMenu.MainMenu_C" _returnvalue))
      (Variables|Widget|SetMainMenuWID _returnvalue_2))))

(event Custom|ShowLoadingScreen
  ;[1 1 1] Engage the spinning circles of Depression
  (Utilities|IsValid (Variables|Default|GetLoadScreenWID)
    (:Is%20Valid
      (UserInterface|Viewport|AddtoViewport (Variables|Default|GetLoadScreenWID) 0))
    (:Is%20Not%20Valid
      (bind _returnvalue (UserInterface|CreateWidget "/Game/Multiplayer/UI/AllLevels/LoadScreen.LoadScreen_C" (Game|GetPlayerController 0)))
      (Variables|Default|SetLoadScreenWID _returnvalue))))

(event Custom|ShowServerMenu
  ;[1 1 1] Serve it to ya
  (bind _returnvalue (UserInterface|CreateWidget "/Game/Multiplayer/UI/MainMenu/ServerMenu.ServerMenu_C" (Game|GetPlayerController 0)))
  (Variables|Widget|SetServerMenuWID _returnvalue))

(event Custom|DestroySessionCaller
  (params (NewParam :type Player%20Controller%20Object%20Reference))
  ;[1 1 1] Destroy the session, handle the supression
  (|DestroySession NewParam))

(event Custom|ShowOptionsMenu
  ;[1 1 1] Woh, slow down, your givin' me too many options
  (Utilities|IsValid (Variables|Widget|GetOptionsMenuWID)
    (:Is%20Valid
      (UserInterface|Viewport|AddtoViewport (Variables|Widget|GetOptionsMenuWID) 0))
    (:Is%20Not%20Valid
      (bind _returnvalue (UserInterface|CreateWidget "/Game/Multiplayer/UI/MainMenu/Options.Options_C" (Game|GetPlayerController 0)))
      (Variables|Widget|SetOptionsMenuWID _returnvalue))))

(event Custom|ShowHostMenu
  ;[1 1 1] Give the host the most, G
  (Utilities|IsValid (Variables|Widget|GetHostMenuWID)
    (:Is%20Valid
      (UserInterface|Viewport|AddtoViewport (Variables|Widget|GetHostMenuWID) 0))
    (:Is%20Not%20Valid
      (bind _returnvalue (UserInterface|CreateWidget "/Game/Multiplayer/UI/MainMenu/HostMenu.HostMenu_C" (Game|GetPlayerController 0)))
      (Variables|Widget|SetHostMenuWID _returnvalue))))

(event Custom|JoinServer
  (params (Session%20Join :type Blueprint%20Session%20Result%20Structure))
  ;[1 1 1] Go on the internet and tell lies
  (CallFunction|ShowLoadingScreen)
  (|JoinSession (Game|GetPlayerController 0) Session%20Join
    (:OnFailure
      (Utilities|DisplayErrorMessage ">You decided to go to bed."))))

(event EventHandleNetworkError
  (params (FailureType :type ENetworkFailure%20Enum :default "NetDriverAlreadyExists") (bIsServer :type Boolean))
  ;[1 1 1] Google Information Collector
  (if (not bIsServer)
    (Utilities|DisplayErrorMessage (CallFunction|NetErrortoString FailureType))))

(event EventHandleTravelError
  (params (FailureType :type ETravelFailure%20Enum :default "NoLevel"))
  ;[1 1 1] Google Information Collector
  (Utilities|DisplayErrorMessage (CallFunction|TravelErrortoString FailureType)))

(fn NetErrortoString
  (params (FailureType :type ENetworkFailure%20Enum :default "NetDriverAlreadyExists"))
  (return ""))

(fn TravelErrortoString
  (params (FailureType :type ETravelFailure%20Enum :default "NoLevel"))
  (return ""))